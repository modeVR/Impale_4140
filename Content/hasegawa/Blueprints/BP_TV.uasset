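; BP_TV is a television actor that shows a channel image or static on a Paper2D sprite.
; A looping timer started at BeginPlay calls the tv event, which sets the sprite from PaperSpriteArray when Channel is below the array length.
; Otherwise Sandstorm alternates two noise sprites on each tick of the timer to animate static.
; ChangeParameter is the setter for Channel, picked up on the next timer call.
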(event `self.ReceiveBeginPlay`
  (`KismetSystemLibrary.K2_SetTimer` null "tv" 0.1 true))

(event `tv`
  (bind _channel (`self.Channel`))
  (bind _returnvalue (`KismetArrayLibrary.Array_Length` (`self.PaperSpriteArray`)))
  (if (and (>= _returnvalue 0) (< _channel _returnvalue))
    (`self.ChangeChannel` _channel)
    (else
      (`self.Sandstorm` (`self.PaperSprite`)))))

(fn `ChangeChannel`
  (params (Channel :type Integer))
  (`PaperSpriteComponent.SetSprite` (`self.PaperSprite`) (`KismetArrayLibrary.Array_Get` (`self.PaperSpriteArray`) Channel)))

(fn `ChangeParameter`
  (params (Channel :type Integer))
  (set `self.Channel` Channel))

(fn `Sandstorm`
  (params (PaperSprite :type "PaperSpriteComponent Object Reference"))
  (bind _flg (`self.flg`))
  (if _flg
    (`PaperSpriteComponent.SetSprite` PaperSprite "/Game/Shihara/Texture/T_suna_Sprite.T_suna_Sprite")
    (else
      (`PaperSpriteComponent.SetSprite` PaperSprite "/Game/Shihara/Texture/T_suna2_Sprite.T_suna2_Sprite")))
  (set `self.flg` (not _flg))
  (return))

(fn `UserConstructionScript`)