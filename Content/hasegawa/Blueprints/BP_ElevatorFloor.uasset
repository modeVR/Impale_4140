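; Elevator floor actor that moves steadily downward each Tick, scaled by Speed and frame time, while fading its movement sound.
; Two nested gates control the motion: Space bar opens the outer one, and the MoveStart event opens the inner one with the move sound and a start camera shake.
; Overlap on Cube or StaticMesh closes the inner gate, swaps to the end sound and plays an arrival shake.
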(event `self.ReceiveBeginPlay`
  (`AudioComponent.Stop` (`self.EndSound`))
  (`AudioComponent.Stop` (`self.MoveSound`))
  (add `self.MoveStart` (delegate `MoveStart_Event`)))

(event `self.ReceiveTick`
  (params (DeltaSeconds :type "Float (single-precision)"))
  (bind _movesound (`self.MoveSound`))
  ;[1 0 0.7438] 稼働中
  (`/Engine/EditorBlueprintResources/StandardMacros.Gate` true :!label _label
    (:`Exit`
      (`/Engine/EditorBlueprintResources/StandardMacros.Gate` false :!label _label_2
        (:`Exit`
          (`AudioComponent.SetVolumeMultiplier` _movesound (- (`AudioComponent.VolumeMultiplier` _movesound) 0.001))
          (`self.K2_SetActorLocation` (`KismetMathLibrary.MakeVector` (.x (`self.K2_GetActorLocation`)) (.y (`self.K2_GetActorLocation`)) (+ (.z (`self.K2_GetActorLocation`)) (* -0.7 (* (`self.Speed`) DeltaSeconds))))))))))

(event `MoveStart_Event`
  ;[1 0 0.7438] 稼働中
  (`AudioComponent.Play` (`self.MoveSound`) 0.0)
  (`PlayerController.ClientStartCameraShake` :`self` (`GameplayStatics.GetPlayerController` 0) :`Shake` "/Game/hasegawa/Blueprints/BP_CameraShale_DownStart.BP_CameraShale_DownStart_C" :`Scale` 1000.0)
  (goto _label_2 :!via `Open`))

(event `スペースバー`
  (goto _label :!via `Open`))

(event `self.Cube.OnComponentBeginOverlap`
  (params (OverlappedComponent :type "PrimitiveComponent Object Reference") (OtherActor :type "Actor Object Reference") (OtherComp :type "PrimitiveComponent Object Reference") (OtherBodyIndex :type Integer) (bFromSweep :type Boolean) (SweepResult :type "HitResult Structure (by ref)"))
  ;[1 0.01256 0.725] 止まる
  (`AudioComponent.Stop` (`self.MoveSound`) :!label _label_3)
  (`AudioComponent.Play` (`self.EndSound`) 0.0)
  (`PlayerController.ClientStartCameraShake` (`GameplayStatics.GetPlayerController` 0) "/Game/hasegawa/Blueprints/BP_CameraShake_DownEnd.BP_CameraShake_DownEnd_C" 1000.0 "CameraLocal" (struct))
  (goto _label_2 :!via `Close`))

(event `self.StaticMesh.OnComponentBeginOverlap`
  (params (OverlappedComponent :type "PrimitiveComponent Object Reference") (OtherActor :type "Actor Object Reference") (OtherComp :type "PrimitiveComponent Object Reference") (OtherBodyIndex :type Integer) (bFromSweep :type Boolean) (SweepResult :type "HitResult Structure (by ref)"))
  (goto _label_3))

(fn `UserConstructionScript`)