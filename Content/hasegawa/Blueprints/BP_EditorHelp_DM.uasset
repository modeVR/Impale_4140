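; BP_EditorHelp_DM is an actor that moves vertically and applies radial damage to its Destructible component when hit.
; While its Z is at or below End's, Tick offsets it further downward by that height gap scaled by Time.
; Damage compounds every tick until the first hit, independent of delta time.
; Each hit uses Damage as base damage, radius and impulse, then sets Swich to stop the growth.
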(event `self.ReceiveTick`
  (params (DeltaSeconds :type "Float (single-precision)"))
  (bind _damage (`self.Damage`))
  (bind (_returnvalue_x _returnvalue_y _returnvalue_z) (`KismetMathLibrary.BreakVector` (- (`self.K2_GetActorLocation`) (`self.End`))))
  (if (<= _returnvalue_z 0.0)
    (`self.K2_AddActorWorldOffset` (`KismetMathLibrary.MakeVector` 0.0 0.0 (/ _returnvalue_z (* (`self.Time`) 2000.0)))))
  (if (not (`self.Swich`))
    (set `self.Damage` (+ _damage (* _damage 0.044)))))

(event `self.ReceiveHit`
  (params (MyComp :type "PrimitiveComponent Object Reference") (Other :type "Actor Object Reference") (OtherComp :type "PrimitiveComponent Object Reference") (bSelfMoved :type Boolean) (HitLocation :type "Vector Structure") (HitNormal :type "Vector Structure") (NormalImpulse :type "Vector Structure") (Hit :type "HitResult Structure (by ref)"))
  (bind _damage (`self.Damage`))
  (`DestructibleComponent.ApplyRadiusDamage` (`self.Destructible`) _damage (`self.K2_GetActorLocation`) _damage _damage false)
  (set `self.Swich` true))

(fn `UserConstructionScript`)