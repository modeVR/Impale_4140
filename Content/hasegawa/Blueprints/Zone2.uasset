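; Zone actor whose sphere grows over time up to a maximum scale, then later shrinks away and destroys itself.
; Tick feeds accumulated time to the sphere's dynamic material and scales it through a gate that closes at the limit.
; The DeleteScale event, rebound every tick, negates the growth rate and reopens both gates, enabling destruction at the minimum scale.
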(event `self.ReceiveBeginPlay`
  (bind _asmaterial_instance_dynamic (cast `MaterialInstanceDynamic` (`PrimitiveComponent.GetMaterial` (`self.Sphere`) 0)))
  (set `self.Material` _asmaterial_instance_dynamic))

(event `self.ReceiveTick`
  (params (DeltaSeconds :type "Float (single-precision)"))
  (bind _nowscale (`self.NowScale`))
  (bind _x (.x _nowscale))
  (bind _output_get (set `self.NowTime` (+ DeltaSeconds (`self.NowTime`))))
  ;[1 0 0.6991] Material Parameter
  (`MaterialInstanceDynamic.SetScalarParameterValue` (`self.Material`) "Time" _output_get)
  (add `self.DeleteScale` (delegate `Custom`))
  (`/Engine/EditorBlueprintResources/StandardMacros.Gate` false :!label _label
    (:`Exit`
      (bind _output_get_2 (set `self.NowScale` (+ _nowscale (* DeltaSeconds (`self.N`)))))
      (`SceneComponent.SetWorldScale3D` (`self.Sphere`) _output_get_2)
      (if (> (`self.LimitMaxScale`) _x)
        (`/Engine/EditorBlueprintResources/StandardMacros.Gate` true :!label _label_2
          (:`Exit`
            (if (not (< (`self.LimitMinScale`) _x))
              (`self.K2_DestroyActor`))))
        (else
          (goto _label :!via `Close`))))))

(event `Custom`
  (set `self.N` (* (`self.N`) -1.0))
  (`|ExecutionSequence`
    (:`then_0`
      (goto _label :!via `Open`))
    (:`then_1`
      (goto _label_2 :!via `Open`))))

(fn `UserConstructionScript`
  (`PrimitiveComponent.CreateDynamicMaterialInstance` (`self.Sphere`) 0 "/Game/hasegawa/Material/M_Wood_Oak_Full.M_Wood_Oak_Full"))