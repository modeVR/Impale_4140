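; Blueprint that moves a referenced Actor along a Spline at a set Speed in an endless loop.
; Each Tick adds frame-scaled Speed to MoveDistance, then sets the Actor's location to the world-space spline point at that distance, leaving rotation untouched.
; GetCurrentLocation wraps distance by modulo of spline length when looping.
; Helpers expose spline length and an end-of-path check, neither called within this Blueprint.
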(event `self.ReceiveTick`
  (params (DeltaSeconds :type "Float (single-precision)"))
  (set `self.MoveDistance` (+ (* DeltaSeconds (`self.Speed`)) (`self.MoveDistance`)))
  (bind _location (`self.GetCurrentLocation` (`self.MoveDistance`) true))
  (`self.K2_SetActorLocation` (`self.Actor`) _location false false))

(fn `GetCurrentLocation`
  (params (Length :type "Float (double-precision)") (Loop :type Boolean))
  (returns (Location :type "Vector Structure"))
  (if Loop
    (set `self.LocalLength` (mod Length (`SplineComponent.GetSplineLength` (`self.Spline`))))
    (else
      (set `self.LocalLength` Length)))
  (return (`SplineComponent.GetLocationAtDistanceAlongSpline` (`self.Spline`) (`self.LocalLength`) "World")))

(fn `GetSplineLength`
  (returns (Length :type "Float (double-precision)"))
  (return (`SplineComponent.GetSplineLength` (`self.Spline`))))

(fn `IsArrived`
  (params (NewParam :type "Float (double-precision)"))
  (returns (NewParam1 :type Boolean))
  (return (>= NewParam (`SplineComponent.GetSplineLength` (`self.Spline`)))))

(fn `UserConstructionScript`)