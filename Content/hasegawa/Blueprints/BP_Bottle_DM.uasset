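; BP_Bottle_DM is a destructible bottle that drops after a delay and breaks on impact.
; Tick records its position for two seconds, pins it there until StartTime, then moves it down with manually computed gravity instead of simulated physics.
; A Hit event applies radius damage scaled by fall speed to the destructible, stops the fall and restarts the timer, so the actor is destroyed one second later.
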(event `self.ReceiveTick`
  (params (DeltaSeconds :type "Float (single-precision)"))
  (bind _output_get (set `self.Timer` (+ (`self.Timer`) DeltaSeconds)))
  (if (`self.Hit`)
    (if (> _output_get 1.0)
      (`/Engine/EditorBlueprintResources/StandardMacros.DoOnce` false
        (:`Completed`
          (`self.K2_DestroyActor`))))
    (elif (> _output_get 2.0)
      ;[1 0.01256 0.725] 落ち始める
      (if (> _output_get (`self.StartTime`))
        ;[1 0 0.7564] 経過時間の保存 ： 速度計算 : 移動
        (set `self.Time` (+ DeltaSeconds (`self.Time`))) ; Set time
        (if (> (`self.Speed`) (`self.MaxSpeed`))
          (set `self.Speed` (`self.MaxSpeed`))
          (else
            (set `self.Speed` (* (* (`self.Time`) (`self.Gravity`)) -1.0)) ; Set speed
          ))
        (`SceneComponent.K2_AddRelativeLocation` (`self.Destructible`) (`KismetMathLibrary.MakeVector` 0.0 0.0 (`self.Speed`)) false false) ; Move
        (else
          (`SceneComponent.K2_SetWorldLocation` (`self.Destructible`) (`self.BeginPosition`) false false)))
      (else
        ;[1 0.07902 0.7487] Set Position
        (set `self.BeginPosition` (`SceneComponent.RelativeLocation` (`self.Destructible`)))))))

(event `self.ReceiveHit`
  (params (MyComp :type "PrimitiveComponent Object Reference") (Other :type "Actor Object Reference") (OtherComp :type "PrimitiveComponent Object Reference") (bSelfMoved :type Boolean) (HitLocation :type "Vector Structure") (HitNormal :type "Vector Structure") (NormalImpulse :type "Vector Structure") (Hit :type "HitResult Structure (by ref)"))
  ;[1 0.004295 0.8003] ダメージを受ける
  (`DestructibleComponent.ApplyRadiusDamage` (`self.Destructible`) (* (`self.Speed`) -1.0) HitLocation 10.0 1.0 true)
  (set `self.Hit` true)
  (`/Engine/EditorBlueprintResources/StandardMacros.DoOnce` false
    (:`Completed`
      (set `self.Timer` 0.0))))

(fn `UserConstructionScript`)