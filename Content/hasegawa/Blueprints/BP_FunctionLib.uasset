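; Blueprint function library with shared helpers for level changes and screen fades.
; SelectLevel maps an enum-like selection to a level name and opens it.
; SelectLevelMP builds a ServerTravel console command from level and game mode lookups with the Listen option, prints it, then executes it for multiplayer travel.
; FadeAction plays a passed-in widget's FadeOut or FadeIn animation according to the Fade value.
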(fn `FadeAction`
  (params (NewParam :type "/Game/hasegawa/Blueprints/WD_RedFade Object Reference") (Fade :type "/Game/hasegawa/Blueprints/BP_Fade Enum"))
  (if (== Fade 0)
    (`UserWidget.PlayAnimation` NewParam (`/Game/hasegawa/Blueprints/WD_RedFade.FadeOut` NewParam) 0.0 1 "Forward" 1.0)
    (else
      (`UserWidget.PlayAnimation` NewParam (`/Game/hasegawa/Blueprints/WD_RedFade.FadeIn` NewParam) 0.0 1 "Forward" 1.0))))

(fn `SelectLevel`
  (params (SelectStarge :type "/Game/hasegawa/Blueprints/BP_Enum Enum"))
  (locals (LevelName :type "Array of Name"))
  (`GameplayStatics.OpenLevel` null (`KismetArrayLibrary.Array_Get` (`local.LevelName`) (`KismetMathLibrary.Conv_ByteToInt` SelectStarge))))

(fn `SelectLevelMP`
  (params (NewParam :type "/Game/Otsuka/BluePrints/ENU_LevelIndex Enum") (Gamemode :type "/Game/Otsuka/BluePrints/ENU_Gamemode Enum"))
  (locals (LevelName :type "Array of Name") (NewLocalVar_0 :type "Array of String"))
  (bind _returnvalue (`KismetStringLibrary.Concat_StrStr` "ServerTravel" " " (`KismetStringLibrary.Conv_NameToString` (`KismetArrayLibrary.Array_Get` (`local.LevelName`) (`KismetMathLibrary.Conv_ByteToInt` NewParam))) (`KismetStringLibrary.Concat_StrStr` "?Listen?Game=" (`KismetArrayLibrary.Array_Get` (`local.NewLocalVar_0`) (`KismetMathLibrary.Conv_ByteToInt` Gamemode)))))
  (`KismetSystemLibrary.PrintString` null _returnvalue)
  (`KismetSystemLibrary.ExecuteConsoleCommand` null _returnvalue))