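; AC_RoomFloor is a room floor actor that rides along with the elevator while their heights overlap.
; At BeginPlay it sets a vertical range from its starting position up by NumMoveRange.
; Each Tick it reads the elevator status from the KUNO game instance and, while the elevator is active inside that range, copies its Z.
; A DoOnce fires the elevator shake event once per entry, resetting outside the range.
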(event `self.ReceiveBeginPlay`
  (`self.FC_SetMovePostion`) ; 変数の初期化
)

(event `self.ReceiveTick`
  (params (DeltaSeconds :type "Float (single-precision)"))
  (bind (_returnvalue_x _returnvalue_y) (`KismetMathLibrary.BreakVector` (`self.K2_GetActorLocation`)))
  (bind (_pos_movemin_x _pos_movemin_y _pos_movemin_z) (`KismetMathLibrary.BreakVector` (`self.Pos_MoveMin`)))
  (bind (_pos_movemax_x _pos_movemax_y _pos_movemax_z) (`KismetMathLibrary.BreakVector` (`self.Pos_MoveMax`)))
  ;[1 1 1] エレベーターとz座標が重なっている時だけ追従する
  (bind _asbp_impale_instance_kuno (cast `/Game/Kuno/BluePrint/BP_ImpaleInstanceKUNO` (`GameplayStatics.GetGameInstance`)))
  (bind _en_elevetorstatus (`/Game/Kuno/BluePrint/BP_ImpaleInstanceKUNO.EN_ElevetorStatus` _asbp_impale_instance_kuno))
  (if (and (!= (break `/Game/Kuno/BluePrint/SR_ElevetorStatus` _en_elevetorstatus) 0) (> (.z (`.Position_5_1917FB49466389D9528EAF9659C67A09` (break `/Game/Kuno/BluePrint/SR_ElevetorStatus` _en_elevetorstatus))) _pos_movemin_z) (< (.z (`.Position_5_1917FB49466389D9528EAF9659C67A09` (break `/Game/Kuno/BluePrint/SR_ElevetorStatus` _en_elevetorstatus))) _pos_movemax_z))
    (set `self.Flg_Move` true)
    (`self.K2_SetActorLocation` (`KismetMathLibrary.MakeVector` _returnvalue_x _returnvalue_y (.z (`.Position_5_1917FB49466389D9528EAF9659C67A09` (break `/Game/Kuno/BluePrint/SR_ElevetorStatus` _en_elevetorstatus)))))
    (`/Engine/EditorBlueprintResources/StandardMacros.DoOnce` false :!label _label
      (:`Completed`
        (`self.EV_ShakeElevetor`)))
    (else
      (set `self.Flg_Move` false)
      (goto _label :!via `Reset`))))

(fn `FC_SetMovePostion`
  (bind _returnvalue (`self.K2_GetActorLocation`))
  (set `self.Pos_MoveMin` _returnvalue)
  (set `self.Pos_MoveMax` (`KismetMathLibrary.MakeVector` (.x _returnvalue) (.y _returnvalue) (+ (.z _returnvalue) (`self.Num_MoveRange`)))))

(fn `UserConstructionScript`)