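; AC_PlayerLogin2D is an actor that reacts to a second player joining, apparently as a 2D login or match-complete notice.
; Tick polls for a valid player controller at index 1, and a DoOnce limits the response to a single run.
; It starts the AC_FripImageActor held in its child actor component, fires the EVTRMachComp dispatcher, then destroys itself after a short delay.
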(event `self.ReceiveTick`
  (params (DeltaSeconds :type "Float (single-precision)"))
  (if (`KismetSystemLibrary.IsValid` (`GameplayStatics.GetPlayerController` 1))
    (`/Engine/EditorBlueprintResources/StandardMacros.DoOnce` false
      (:`Completed`
        (`/Game/Kuno/BluePrint/AC_FripImageActor.EV_Start` (cast `/Game/Kuno/BluePrint/AC_FripImageActor` (`ChildActorComponent.ChildActor` (`self.AC_FripImageActor`)) :!pure true))
        (`/Engine/EditorBlueprintResources/StandardMacros.DoOnce` false
          (:`Completed`
            (`self.EV_TR_MachComp`)
            (`KismetSystemLibrary.Delay` 5.0)
            (`self.K2_DestroyActor`)))))))

(fn `UserConstructionScript`)