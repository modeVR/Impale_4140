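; AC_DragTR2D is a tips actor that reacts to the press state of its child AC_Light2D, driving a spotlight and an explanation sprite.
; Every tick while pressed, it snaps the SpotLight to player controller 0's location and camera rotation, with identical authority and remote branches.
; It also switches the 説明文02 sprite to the default lit material when pressed, and back to the alpha material otherwise.
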(event `self.ReceiveTick`
  (params (DeltaSeconds :type "Float (single-precision)"))
  (bind _returnvalue (`GameplayStatics.GetPlayerController` 0))
  (bind _returnvalue_2 (`GameplayStatics.GetPlayerController` 0))
  (bind _spotlight (`self.SpotLight`))
  (bind _asac_light_2d (cast `/Game/Kuno/BluePrint/Tips/AC_Light2D` (`ChildActorComponent.ChildActor` (`self.AC_Light2D`))))
  (if (`/Game/Otsuka/BaseBluePrint/BBP_ClickableObject.PressFlg` _asac_light_2d)
    (`/Engine/EditorBlueprintResources/ActorMacros.Switch Has Authority`
      (:`Authority`
        (`SceneComponent.K2_SetWorldRotation` _spotlight (`self.K2_GetActorRotation` (`PlayerController.PlayerCameraManager` _returnvalue_2)) false false)
        (`SceneComponent.K2_SetWorldLocation` _spotlight (`self.K2_GetActorLocation` _returnvalue_2) false false))
      (:`Remote`
        (`SceneComponent.K2_SetWorldRotation` _spotlight (`self.K2_GetActorRotation` (`PlayerController.PlayerCameraManager` _returnvalue)) false false)
        (`SceneComponent.K2_SetWorldLocation` _spotlight (`self.K2_GetActorLocation` _returnvalue) false false)))
    (`PrimitiveComponent.SetMaterial` (`self.説明文02_Sprite`) 0 "/Paper2D/DefaultLitSpriteMaterial.DefaultLitSpriteMaterial")
    (else
      (`PrimitiveComponent.SetMaterial` (`self.説明文02_Sprite`) 0 "/Game/Kuno/Material/MT_paper2dAlpha.MT_paper2dAlpha"))))

(fn `UserConstructionScript`)