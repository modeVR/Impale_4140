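; Actor that flips between two sprite images, toggled by a click when FlgClick is set or by EV_Start.
; Construction assigns both sprites, hides the second and scales timeline speed by the inverse of FrameLate.
; A zero FrameLate swaps alpha instantly; otherwise a DoOnce-guarded timeline crossfades forward or in reverse, and EV_Stop halts it.
; Empty begin and finish events serve as hooks for each flip direction.
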(event `self.OnClick`
  (bind _tgl_click (`self.tgl_click`))
  (if (`self.flg_Click`)
    (if (== (`self.FrameLate`) 0.0) :!label _label
      (if _tgl_click
        (`self.EV_FripBeginSecond`)
        (else
          (`self.EV_FripBeginFirst`)))
      (`PaperSpriteComponent.SetSpriteColor` (`self.FripImage02`) (make `LinearColor` 1.0 1.0 1.0 (`KismetMathLibrary.Conv_BoolToDouble` (not _tgl_click))))
      (`PaperSpriteComponent.SetSpriteColor` (`self.FripImage01`) (make `LinearColor` 1.0 1.0 1.0 (`KismetMathLibrary.Conv_BoolToDouble` _tgl_click)))
      (set `self.tgl_click` (not (`self.tgl_click`)))
      (if (== (`self.tgl_click`) true) :!label _label_2
        (`self.EV_FripFinishFirst`)
        (else
          (`self.EV_FripFnishSecond`)))
      (else
        (`/Engine/EditorBlueprintResources/StandardMacros.DoOnce` false :!label _label_3
          (:`Completed`
            (if _tgl_click
              (`self.EV_FripBeginSecond`)
              (bind (_direction `_新規track_0`) (`Timeline|タイムライン_0` :!via `Reverse` :!label _label_4)
                (:`Update`
                  (`PaperSpriteComponent.SetSpriteColor` (`self.FripImage02`) (make `LinearColor` 1.0 1.0 1.0 `_新規track_0`))
                  (`PaperSpriteComponent.SetSpriteColor` (`self.FripImage01`) (make `LinearColor` 1.0 1.0 1.0 (- 1.0 `_新規track_0`)))
                  (goto _label_2))
                (:`Finished`
                  (set `self.tgl_click` (not (`self.tgl_click`)))
                  (goto _label_3 :!via `Reset`)))
              (else
                (`self.EV_FripBeginFirst`)
                (goto _label_4)))))))))

(event `EV_Start`
  (goto _label))

(event `EV_Stop`
  (goto _label_4 :!via `Stop`))

(event `EV_FripBeginFirst`)

(event `EV_FripBeginSecond`)

(event `EV_FripFinishFirst`)

(event `EV_FripFnishSecond`)

(fn `UserConstructionScript`
  (bind _fripimage (`self.FripImage`))
  (bind _framelate (`self.FrameLate`))
  (bind _fripimage02 (`self.FripImage02`))
  (`PaperSpriteComponent.SetSpriteColor` _fripimage02 (make `LinearColor` 1.0 1.0 1.0 0.0))
  (`PaperSpriteComponent.SetSprite` _fripimage02 (`KismetArrayLibrary.Array_Get` _fripimage 1))
  (`PaperSpriteComponent.SetSprite` (`self.FripImage01`) (`KismetArrayLibrary.Array_Get` _fripimage))
  (if (not (== _framelate 0.0))
    (`TimelineComponent.SetPlayRate` (`self.タイムライン_0`) (/ 1.0 _framelate))))