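; BP_ImpaleInstanceKUNO maintains SpawnBlockList, a list of puzzle block spawn records.
; EV_AddSpawnBlockList passes a record to MC_AddSpawnBlockList, which searches for a valid matching puzzle block reference.
; A match with a different spawn point gets its spawn data overwritten, while an equal one stays unchanged and unmatched records are appended.
; EV_SetSpawnBlockList is an empty stub.
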(event `EV_AddSpawnBlockList`
  (params (STR_PBSpawnData :type "/Game/Otsuka/Actors/STR_PBSpawnData Structure (by ref)"))
  (`self.MC_AddSpawnBlockList` STR_PBSpawnData))

(event `EV_SetSpawnBlockList`)