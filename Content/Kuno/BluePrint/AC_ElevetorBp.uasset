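; Elevator actor that publishes its position to the game instance and can shake on demand.
; Every tick it writes its current location into the elevator status on BP_ImpaleInstanceKUNO, keeping the existing state.
; EV_Shake saves the start position, then a timeline scaled to the requested duration offsets X by the swing width.
; A flag ignores new shake calls until the timeline finishes.
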(event `self.ReceiveBeginPlay`)

(event `self.ReceiveTick`
  (params (DeltaSeconds :type "Float (single-precision)"))
  (bind _asbp_impale_instance_kuno (cast `/Game/Kuno/BluePrint/BP_ImpaleInstanceKUNO` (`GameplayStatics.GetGameInstance`)))
  (bind _en_elevetorstatus_state (break `/Game/Kuno/BluePrint/SR_ElevetorStatus` (`/Game/Kuno/BluePrint/BP_ImpaleInstanceKUNO.EN_ElevetorStatus` _asbp_impale_instance_kuno)))
  (set `/Game/Kuno/BluePrint/BP_ImpaleInstanceKUNO.EN_ElevetorStatus` (make `/Game/Kuno/BluePrint/SR_ElevetorStatus` _en_elevetorstatus_state (`self.K2_GetActorLocation`)) _asbp_impale_instance_kuno))

(event `EV_Shake`
  (params (ShakeTime :type "Float (double-precision)") (SwingWidth :type "Float (double-precision)"))
  (bind (_returnvalue_x _returnvalue_y _returnvalue_z) (`KismetMathLibrary.BreakVector` (`self.K2_GetActorLocation`)))
  (bind _pos_evshakebaf_x (`KismetMathLibrary.BreakVector` (`self.pos_EVShakeBaf`)))
  (if (not (`self.flg_EVShakeNow`))
    (set `self.flg_EVShakeNow` true)
    (set `self.pos_EVShakeBaf` (`self.K2_GetActorLocation`))
    (`TimelineComponent.SetPlayRate` (`self.ShakeTimeLine`) (/ 1.0 ShakeTime))
    (bind (_direction `_新規track_0`) (`Timeline|ShakeTimeLine`)
      (:`Update`
        (`self.K2_SetActorLocation` (`KismetMathLibrary.MakeVector` (+ (* SwingWidth `_新規track_0`) _pos_evshakebaf_x) _returnvalue_y _returnvalue_z)))
      (:`Finished`
        (set `self.flg_EVShakeNow` false)))))

(fn `UserConstructionScript`)