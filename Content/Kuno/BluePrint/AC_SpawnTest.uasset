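; AC_SpawnTest is a test Blueprint that creates AC_PBStartBlock instances in three different ways.
; BeginPlay spawns one as a standalone actor at its own transform and adds another through a Child Actor Component offset 300 units along X.
; The Construction Script adds a third Child Actor Component of the same class, offset 600 units along X.
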(event `self.ReceiveBeginPlay`
  (`|SpawnActorFromClass` "/Game/Otsuka/Actors/PuzzleBlock/AC_PBStartBlock.AC_PBStartBlock_C" (`self.GetTransform`) "Undefined" "OverrideRootScale")
  (bind _returnvalue (`AddComponent|NODE_AddChildActorComponent-0` :`RelativeTransform` (`KismetMathLibrary.MakeTransform` (`KismetMathLibrary.MakeVector` 300.0) (struct) (1.0 1.0 1.0))))
  (`ChildActorComponent.SetChildActorClass` _returnvalue "/Game/Otsuka/Actors/PuzzleBlock/AC_PBStartBlock.AC_PBStartBlock_C"))

(fn `UserConstructionScript`
  (bind _returnvalue (`AddComponent|NODE_AddChildActorComponent-1` :`RelativeTransform` (`KismetMathLibrary.MakeTransform` (`KismetMathLibrary.MakeVector` 600.0) (struct) (1.0 1.0 1.0))))
  (`ChildActorComponent.SetChildActorClass` _returnvalue "/Game/Otsuka/Actors/PuzzleBlock/AC_PBStartBlock.AC_PBStartBlock_C"))