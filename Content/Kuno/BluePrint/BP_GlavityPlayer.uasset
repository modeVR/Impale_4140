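; VR-capable player with camera look that enables the HMD at start and interacts with objects by gaze.
; Each Tick, a Visibility line trace along the camera's forward vector finds BBP_ClickableObject targets, tracking hover state and sending eye-track and leave calls.
; Click input forwards press and release to the gazed object, while the A key calls CallDeadPlayer.
; EV_Shake uses a timeline to offset the actor along world X, guarded against overlapping shakes.
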(event `InputAxis|CameraRotationYaw`
  (params (AxisValue :type "Float (single-precision)"))
  (`SceneComponent.K2_AddWorldRotation` (`self.Camera`) (`KismetMathLibrary.MakeRotator` 0.0 0.0 AxisValue) false false))

(event `InputAxis|CameraRotationPitch`
  (params (AxisValue :type "Float (single-precision)"))
  (`SceneComponent.K2_AddLocalRotation` (`self.Camera`) (`KismetMathLibrary.MakeRotator` 0.0 AxisValue) false false))

(event `HMDActivation`
  ;[1 1 1] HMDをアクティベーションするイベント
  (`HeadMountedDisplayFunctionLibrary.EnableHMD` true)
  (if (`HeadMountedDisplayFunctionLibrary.IsHeadMountedDisplayEnabled`)
    (`KismetSystemLibrary.ExecuteConsoleCommand` "stereo on")))

(event `self.ReceiveBeginPlay`
  (`self.HMDActivation`))

(event `self.ReceiveTick`
  (params (DeltaSeconds :type "Float (single-precision)"))
  (bind _hitobject (`self.HitObject`))
  (bind _hitobject_2 (`self.HitObject`))
  (bind _returnvalue (`SceneComponent.K2_GetComponentLocation` (`self.Camera`)))
  ;[1 1 1] ライントレースの発動
  (bind _outhit (`KismetSystemLibrary.LineTraceSingle` :`Start` _returnvalue :`End` (+ _returnvalue (* (`SceneComponent.GetForwardVector` (`self.Camera`)) (`self.LookDistance`))) :`TraceChannel` "TraceTypeQuery1" :`DrawDebugType` "ForOneFrame"))
  ;[1 1 1] 視線の先のオブジェクトがClick可能オブジェクトか？
  (bind _asbbp_clickable_object (cast `/Game/Otsuka/BluePrints/BBP_ClickableObject` (`.HitActor` (`GameplayStatics.BreakHitResult` _outhit)))
    (:`then`
      (`/Engine/EditorBlueprintResources/StandardMacros.IsValid` (`self.HitObject`)
        (:`Is Valid`
          (if (not (!= _asbbp_clickable_object _hitobject))
            (`/Game/Otsuka/BluePrints/BBP_ClickableObject.LeaveClick` _hitobject)
            (bind _output_get (set `self.HitObject` _asbbp_clickable_object :!label _label))))
        (:`Is Not Valid`
          (goto _label)))
      (`/Game/Otsuka/BluePrints/BBP_ClickableObject.ReciveEyeTrack` _output_get)
      (set `self.hitClickable` true))
    (:`CastFailed`
      (set `self.hitClickable` false)
      (`/Engine/EditorBlueprintResources/StandardMacros.IsValid` _hitobject_2
        (:`Is Valid`
          (`/Game/Otsuka/BluePrints/BBP_ClickableObject.LeaveClick` _hitobject_2))))))

(event `InputAction|Click`
  (params (Key :type "Key Structure" :default "AnyKey"))
  ;[1 1 1] クリックボタンを操作時の動作
  (:`Pressed`
    (`self.IsHitClickable`
      (:`true`
        (`/Game/Otsuka/BluePrints/BBP_ClickableObject.OnClick` (`self.HitObject`)))))
  (:`Released`
    (`self.IsHitClickable`
      (:`true`
        (`/Game/Otsuka/BluePrints/BBP_ClickableObject.LeaveClick` (`self.HitObject`))))))

(event `Key|A`
  (params (Key :type "Key Structure" :default "AnyKey"))
  (:`Pressed`
    (`self.DeadPlayer`)))

(event `EV_Shake`
  (params (ShakeTime :type "Float (double-precision)") (SwingWidth :type "Float (double-precision)"))
  (bind (_returnvalue_x _returnvalue_y _returnvalue_z) (`KismetMathLibrary.BreakVector` (`self.K2_GetActorLocation`)))
  (bind _pos_evshakebaf_x (`KismetMathLibrary.BreakVector` (`self.pos_EVShakeBaf`)))
  ;[1 1 1] シェイク
  (if (not (`self.flg_EVShakeNow`))
    (set `self.flg_EVShakeNow` true)
    (set `self.pos_EVShakeBaf` (`self.K2_GetActorLocation`))
    (`TimelineComponent.SetPlayRate` (`self.ShakeTimeLine`) (/ 1.0 ShakeTime))
    (bind (_direction `_新規track_0`) (`Timeline|ShakeTimeLine` :!via `PlayFromStart`)
      (:`Update`
        (`self.K2_SetActorLocation` (`KismetMathLibrary.MakeVector` (+ (* SwingWidth `_新規track_0`) _pos_evshakebaf_x) _returnvalue_y _returnvalue_z)))
      (:`Finished`
        (set `self.flg_EVShakeNow` false)))))

(fn `UserConstructionScript`)