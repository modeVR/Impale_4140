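; AC_Button is a pressable button actor whose top part moves along its vertical axis on click and release.
; BeginPlay caches the top component's resting relative location.
; OnClick plays a timeline that adds its TopYCoord track to the cached Z, despite the track's name, and LeaveClick reverses it to return the top.
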(event `self.ReceiveBeginPlay`
  (bind _returnvalue_location (`KismetMathLibrary.BreakTransform` (`SceneComponent.GetRelativeTransform` (`self.but_Top`))))
  (set `self.DefButCoord` _returnvalue_location))

(event `self.OnClick`
  (bind (_defbutcoord_x _defbutcoord_y _defbutcoord_z) (`KismetMathLibrary.BreakVector` (`self.DefButCoord`)))
  (bind _returnvalue (`SceneComponent.GetRelativeTransform` (`self.but_Top`)))
  (bind (_direction _topycoord) (`Timeline|Timeline` :!label _label)
    (:`Update`
      (`SceneComponent.K2_SetRelativeLocation` (`self.but_Top`) (`KismetMathLibrary.MakeVector` (.x (.location _returnvalue)) (.y (.location _returnvalue)) (+ _topycoord _defbutcoord_z)) false false))))

(event `self.LeaveClick`
  (goto _label :!via `Reverse`))

(fn `UserConstructionScript`)