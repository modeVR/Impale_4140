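; VR player with a camera-driven gaze cursor for interacting with BBP_ClickableObject actors.
; It enables the HMD at start, then line-traces from the camera each tick, passing the hit point to the gazed object and releasing it when lost.
; Click input presses or releases that object.
; It also handles camera rotation, a timeline-driven X-axis shake, a screenshot key, and a death sound and call on any capsule overlap or debug key.
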(event `InputAxis|CameraRotationYaw`
  (params (AxisValue :type "Float (single-precision)"))
  ;[1 1 1] カメラをヨー回転
  (`SceneComponent.K2_AddWorldRotation` (`self.Camera`) (`KismetMathLibrary.MakeRotator` 0.0 0.0 AxisValue) false false))

(event `Key|P`
  (params (Key :type "Key Structure" :default "AnyKey"))
  (:`Pressed`
    (`KismetSystemLibrary.ExecuteConsoleCommand` "HighResShot 4677x6622")))

(event `InputAxis|CameraRotationPitch`
  (params (AxisValue :type "Float (single-precision)"))
  ;[1 1 1] カメラをピッチ軸回転
  (`SceneComponent.K2_AddLocalRotation` (`self.Camera`) (`KismetMathLibrary.MakeRotator` 0.0 AxisValue) false false))

(event `HMDActivation`
  ;[1 1 1] HMDをアクティベーションするイベント
  (`HeadMountedDisplayFunctionLibrary.EnableHMD` true)
  (if (`HeadMountedDisplayFunctionLibrary.IsHeadMountedDisplayEnabled`)
    (`KismetSystemLibrary.ExecuteConsoleCommand` "stereo on")))

(event `self.ReceiveBeginPlay`
  (`self.HMDActivation`))

(event `self.ReceiveTick`
  (params (DeltaSeconds :type "Float (single-precision)"))
  ;[1 1 1] 視線の先の物の判別
  (bind _hitresult (`self.LinetraceByPlayer` "TraceTypeQuery1"))
  (`self.IsClickableObject` _hitresult))

(event `HitClickableObject`
  (bind _hitobject (`self.HitObject`))
  (bind _t_hitobject (`self.t_hitObject`))
  ;[1 1 1] 視線の先のオブジェクトがClick可能オブジェクトか？
  (`/Engine/EditorBlueprintResources/StandardMacros.IsValid` (`self.HitObject`)
    (:`Is Valid`
      (if (== _t_hitobject _hitobject)
        _
        (elif (not (`/Game/Otsuka/BaseBluePrint/BBP_ClickableObject.PressFlg` _hitobject))
          (`/Game/Otsuka/BaseBluePrint/BBP_ClickableObject.LeaveClick` _hitobject)
          (bind _output_get (set `self.HitObject` _t_hitobject :!label _label)))))
    (:`Is Not Valid`
      (goto _label)))
  (`/Game/Otsuka/BaseBluePrint/BBP_ClickableObject.ReciveEyeTrack` _output_get (`self.t_impactPoint`))
  (set `self.hitClickable` true))

(event `InputAction|Click`
  (params (Key :type "Key Structure" :default "AnyKey"))
  (bind _hitobject (`self.HitObject`))
  (bind _hitobject_2 (`self.HitObject`))
  ;[1 1 1] クリックボタンを操作時の動作
  (:`Pressed`
    (`self.IsHitClickable`
      (:`true`
        (`/Engine/EditorBlueprintResources/StandardMacros.IsValid` _hitobject_2
          (:`Is Valid`
            (`/Game/Otsuka/BaseBluePrint/BBP_ClickableObject.OnClick` _hitobject_2)
            (set `self.Clickflg` true))))))
  (:`Released`
    (`self.IsHitClickable`
      (:`true`
        (`/Engine/EditorBlueprintResources/StandardMacros.IsValid` _hitobject
          (:`Is Valid`
            (`/Game/Otsuka/BaseBluePrint/BBP_ClickableObject.LeaveClick` _hitobject)
            (set `self.Clickflg` false)))))))

(event `Key|A`
  (params (Key :type "Key Structure" :default "AnyKey"))
  (:`Pressed`
    (`KismetSystemLibrary.PrintString` "Hello" :!label _label_2)
    (`/Game/Otsuka/BluePrints/ACC_SoundCompornent.PlaySound` (`self.dead`) (0.0 0.0 0.0))
    (`self.DeadPlayer`)))

(event `NotHitClickableObject`
  (bind _hitobject (`self.HitObject`))
  ;[1 1 1] clickableObjectではなかった時の処理
  (`/Engine/EditorBlueprintResources/StandardMacros.IsValid` _hitobject
    (:`Is Valid`
      (`/Game/Otsuka/BaseBluePrint/BBP_ClickableObject.LeaveClick` _hitobject)
      (set `self.hitClickable` false)
      (set `self.HitObject` null))))

(event `self.CapsuleComponent.OnComponentBeginOverlap`
  (params (OverlappedComponent :type "PrimitiveComponent Object Reference") (OtherActor :type "Actor Object Reference") (OtherComp :type "PrimitiveComponent Object Reference") (OtherBodyIndex :type Integer) (bFromSweep :type Boolean) (SweepResult :type "HitResult Structure (by ref)"))
  (goto _label_2))

(event `EV_Shake`
  (params (ShakeTime :type "Float (double-precision)") (SwingWidth :type "Float (double-precision)"))
  (bind (_returnvalue_x _returnvalue_y _returnvalue_z) (`KismetMathLibrary.BreakVector` (`self.K2_GetActorLocation`)))
  (bind _pos_evshakebaf_x (`KismetMathLibrary.BreakVector` (`self.pos_EVShakeBaf`)))
  ;[1 1 1] シェイク
  (if (not (`self.flg_EVShakeNow`))
    (set `self.flg_EVShakeNow` true)
    (set `self.pos_EVShakeBaf` (`self.K2_GetActorLocation`))
    (`TimelineComponent.SetPlayRate` (`self.Shake TimeLine`) (/ 1.0 ShakeTime))
    (bind (_direction `_新規track_0`) (`Timeline|Shake TimeLine` :!via `PlayFromStart`)
      (:`Update`
        (`self.K2_SetActorLocation` (`KismetMathLibrary.MakeVector` (+ (* SwingWidth `_新規track_0`) _pos_evshakebaf_x) _returnvalue_y _returnvalue_z)))
      (:`Finished`
        (set `self.flg_EVShakeNow` false)))))

(fn `IsClickableObject`
  (params (HitResult :type "HitResult Structure"))
  (returns (IsClickable :type Boolean))
  (locals (t_IsClickable :type Boolean))
  (bind (_bblockinghit _binitialoverlap _time _location _impactpoint _normal _impactnormal _physmat _hitactor) (`GameplayStatics.BreakHitResult` HitResult))
  ;[1 1 1] 視線の先のオブジェクトがClick可能オブジェクトか？
  (set `self.t_impactPoint` _impactpoint)
  (bind _asbbp_clickable_object (cast `/Game/Otsuka/BaseBluePrint/BBP_ClickableObject` _hitactor)
    (:`then`
      (set `self.t_hitObject` _asbbp_clickable_object)
      (`self.HitClickableObject`)
      (set `local.t_IsClickable` true))
    (:`CastFailed`
      (`self.NotHitClickableObject`)
      (set `local.t_IsClickable` false)))
  (return (`local.t_IsClickable`)))

(fn `LinetraceByPlayer`
  (params (TraceChannel :type "ETraceTypeQuery Enum"))
  (returns (HitResult :type "HitResult Structure"))
  (bind _returnvalue (`SceneComponent.K2_GetComponentLocation` (`self.Camera`)))
  ;[1 1 1] ライントレースの発動
  (bind _outhit (`KismetSystemLibrary.LineTraceSingle` :`Start` _returnvalue :`End` (+ _returnvalue (* (`SceneComponent.GetForwardVector` (`self.Camera`)) (`self.LookDistance`))) :`TraceChannel` TraceChannel :`DrawDebugType` "ForOneFrame"))
  (return _outhit))

(fn `UserConstructionScript`)