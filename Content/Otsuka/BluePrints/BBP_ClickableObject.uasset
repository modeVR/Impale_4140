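; BBP_ClickableObject is a clickable-object Blueprint that fires an Action after enough sufficiently long presses.
; OnClick starts Tick to time the hold and print it for debugging; LeaveClick stops Tick and counts presses meeting RequiredPressSecond.
; Action runs on qualifying releases once the count, which is never reset here, reaches RequiredPressCount.
; Action and ReciveEyeTrack are empty here.
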(event `self.ReceiveTick`
  (params (DeltaSeconds :type "Float (single-precision)"))
  (if (`self.PressFlg`)
    (bind _output_get (set `self.pressSecond` (+ (`self.pressSecond`) DeltaSeconds)))
    (`KismetSystemLibrary.PrintString` (`KismetStringLibrary.Concat_StrStr` "Press SEcond =" (`KismetStringLibrary.Conv_DoubleToString` _output_get)) true true (struct :`G` 0.66 :`B` 1.0 :`A` 1.0) 0.0)))

(fn `Action`)

(fn `LeaveClick`
  (set `self.PressFlg` false)
  (`self.SetActorTickEnabled` false)
  (if (>= (`self.pressSecond`) (`self.RequiredPressSecond`))
    (bind _result (`/Engine/EditorBlueprintResources/StandardMacros.IncrementInt` (`self.pressCount`))
      (:`  `
        (if (>= _result (`self.requiredPressCount`))
          (`self.Action`))))))

(fn `OnClick`
  (`self.SetActorTickEnabled` true)
  (set `self.PressFlg` true)
  (set `self.pressSecond` 0.0))

(fn `ReciveEyeTrack`)

(fn `UserConstructionScript`)