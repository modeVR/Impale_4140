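; Player Blueprint for dragging and dropping puzzle blocks by aiming the camera and holding Click.
; Each tick a line trace finds the clickable object and caches it as the current puzzle block.
; Pressing Click notifies the object and attaches it to the SpringArm; releasing notifies and detaches it.
; While held, a second trace on a separate channel finds vacuum (snap) points and passes the hit one to the block.
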(event `self.ReceiveTick`
  (params (DeltaSeconds :type "Float (single-precision)"))
  (set `self.ATime` (`.PartialSeconds` (`GameplayStatics.GetAccurateRealTime`)))
  (bind _hitresult (`self.LinetraceByPlayer` "TraceTypeQuery1"))
  (bind _isclickable (`self.IsClickableObject` _hitresult))
  (if _isclickable
    (bind _asac_puzzle_block (cast `/Game/Otsuka/Actors/PuzzleBlock/AC_PuzzleBlock` (`self.HitObject`)))
    (set `self.hitPuzzleBlock` _asac_puzzle_block)
    (if (`self.Clickflg`)
      ;[1 1 1] 吸着点へのライントレース
      (bind _hitresult_2 (`self.LinetraceByPlayer` "TraceTypeQuery3"))
      (bind (_bblockinghit _binitialoverlap _time _location _impactpoint _normal _impactnormal _physmat _hitactor) (`GameplayStatics.BreakHitResult` _hitresult_2))
      (if _bblockinghit
        (bind _asac_vacuum_point (cast `/Game/Otsuka/Actors/VacuumPoint/AC_VacuumPoint` _hitactor))
        (`/Game/Otsuka/Actors/PuzzleBlock/AC_PuzzleBlock.ChangeLasthitVacuumPoint` (`self.hitPuzzleBlock`) _asac_vacuum_point)))))

(event `InputAction|Click`
  (params (Key :type "Key Structure" :default "AnyKey"))
  (bind _hitobject (`self.HitObject`))
  (bind _asbbp_drag_and_drop_object (cast `/Game/Otsuka/BaseBluePrint/BBP_DragAndDropObject` _hitobject :!pure true))
  (:`Pressed`
    (`/Engine/EditorBlueprintResources/StandardMacros.IsValid` _hitobject
      (:`Is Valid`
        (`self.IsHitclickable`
          (:`true`
            (`/Game/Otsuka/BaseBluePrint/BBP_ClickableObject.OnClick` _hitobject)
            (`/Game/Otsuka/BaseBluePrint/BBP_DragAndDropObject.AttachThis` _asbbp_drag_and_drop_object (`self.SpringArm`))
            (set `self.Clickflg` true))))))
  (:`Released`
    (`/Engine/EditorBlueprintResources/StandardMacros.IsValid` _hitobject
      (:`Is Valid`
        (`self.IsHitclickable`
          (:`true`
            (`/Game/Otsuka/BaseBluePrint/BBP_ClickableObject.LeaveClick` _hitobject)
            (`/Game/Otsuka/BaseBluePrint/BBP_DragAndDropObject.DetachThis` _asbbp_drag_and_drop_object)
            (set `self.Clickflg` false)))))))

(fn `multiLinetraceByPlayer`
  (returns (OutHits :type "Array of HitResult Structure"))
  (bind _returnvalue (`SceneComponent.K2_GetComponentLocation` (`self.Camera`)))
  ;[1 1 1] ライントレースの発動
  (bind _outhits (`KismetSystemLibrary.LineTraceMulti_NEW` :`Start` _returnvalue :`End` (+ _returnvalue (* (`SceneComponent.GetForwardVector` (`self.Camera`)) (`self.LookDistance`))) :`TraceChannel` "TraceTypeQuery1" :`DrawDebugType` "ForOneFrame"))
  (return _outhits))

(fn `UserConstructionScript`
  (`parent.UserConstructionScript`))