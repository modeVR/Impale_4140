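; Spline-driven tape actor that lays a line mesh along an editable spline, built entirely in the construction script.
; For each pair of consecutive spline points, AddTrackElement spawns a spline mesh component using the local-space locations and tangents as start and end.
; Each segment gets the same roll and unit scale at both ends, and the spline is left open.
; The event graph holds no active logic.
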(event EventBeginPlay)

(event Collision|EventActorBeginOverlap
  (params (OtherActor :type Actor%20Object%20Reference)))

(event EventTick
  (params (DeltaSeconds :type Float%20%28single-precision%29)))

(fn ConstructionScript
  (Utilities|FlowControl|Sequence
    (:then_0
      (Variables|Default|SetNumberOfSplinePoint (Spline|GetNumberOfSplinePoints (Variables|Default|GetSpline))))
    (:then_1
      (for _index (range 0 (- (Variables|Default|GetNumberOfSplinePoint) 2))
        (bind _output_get (Variables|Default|SetCurrentLoopIndex _index))
        (CallFunction|AddTrackElement (Variables|Default|GetLineMesh) _output_get)))))

(fn AddTrackElement
  (params (PlaceMesh :type Static%20Mesh%20Object%20Reference) (index :type Integer))
  (LocalVariables|SetLocalCurrentTrackPoint index)
  (LocalVariables|SetLocalNextTrackPoint (Math|Integer|%(Integer) (+ index 1) (Variables|Default|GetNumberOfSplinePoint)))
  (LocalVariables|SetLocalTrackElementMesh PlaceMesh)
  (Utilities|FlowControl|Sequence
    (:then_0
      (LocalVariables|SetLocalStartPosition (.Location (Spline|GetLocationandTangentatSplinePoint (Variables|Default|GetSpline) (LocalVariables|GetLocalCurrentTrackPoint) "Local")))
      (LocalVariables|SetLocalStartTangent (.Tangent (Spline|GetLocationandTangentatSplinePoint (Variables|Default|GetSpline) (LocalVariables|GetLocalCurrentTrackPoint) "Local")))
      (LocalVariables|SetLocalEndPosition (.Location (Spline|GetLocationandTangentatSplinePoint (Variables|Default|GetSpline) (LocalVariables|GetLocalNextTrackPoint) "Local")))
      (LocalVariables|SetLocalEndTangent (.Tangent (Spline|GetLocationandTangentatSplinePoint (Variables|Default|GetSpline) (LocalVariables|GetLocalNextTrackPoint) "Local"))))
    (:then_1
      (bind _returnvalue (AddComponent|AddSplineMeshComponent false))
      (LocalVariables|SetLocalCurrentSplineMesh _returnvalue)
      (Components|StaticMesh|SetStaticMesh (LocalVariables|GetLocalCurrentSplineMesh) (LocalVariables|GetLocalTrackElementMesh))
      (SplineMesh|SetStartandEnd (LocalVariables|GetLocalCurrentSplineMesh) (LocalVariables|GetLocalStartPosition) (LocalVariables|GetLocalStartTangent) (LocalVariables|GetLocalEndPosition) (LocalVariables|GetLocalEndTangent) true :!class /Script/Engine.SplineMeshComponent)
      (Utilities|FlowControl|Sequence
        (:then_0
          (Class|SplineMeshComponent|SetStartRoll (LocalVariables|GetLocalCurrentSplineMesh) (Variables|Default|GetFlortRoll) true)
          (Class|SplineMeshComponent|SetEndRoll (LocalVariables|GetLocalCurrentSplineMesh) (Variables|Default|GetFlortRoll) true))
        (:then_1
          (SplineMesh|SetStartScale (LocalVariables|GetLocalCurrentSplineMesh) "(X=1.000,Y=1.000)" true :!class /Script/Engine.SplineMeshComponent)
          (SplineMesh|SetEndScale (LocalVariables|GetLocalCurrentSplineMesh) "(X=1.000,Y=1.000)" true :!class /Script/Engine.SplineMeshComponent))))))