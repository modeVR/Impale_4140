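; AC_Lever is a lever actor that the player pulls by holding left mouse when it receives eye-track events.
; While GameInstance event flag 0 is set, it calls OnClick on press, otherwise LeaveClick.
; PressAction's timeline pitches the handle, notifying the level through CallEVActiveLeverToLevel at -90 degrees or below.
; LeaveClick reverses the timeline, locking out further input once Click is set at exactly -90.
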(event `self.ReceiveBeginPlay`)

(event `self.ReciveEyeTrack`
  (if (not (`self.Clicked`))
    (bind _asgi_game_instance (cast `/Game/otsuka/GI_GameInstance` (`GameplayStatics.GetGameInstance`)))
    (if (`KismetArrayLibrary.Array_Get` (`/Game/otsuka/GI_GameInstance.EventFlg` _asgi_game_instance))
      (if (`PlayerController.IsInputKeyDown` (`GameplayStatics.GetPlayerController` 0) "LeftMouseButton")
        (`self.OnClick`)
        (else
          (`self.LeaveClick`))))))

(event `self.Action`
  ;[1 1 1] レバーが動き切った時の動作
  (`self.EVActiveLeverToLevel`))

(event `self.PressAction`
  ;[1 1 1] クリックするとレバーが動くよ！
  (bind (_direction _rotationtimer) (`Timeline|タイムライン_0` :!label _label)
    (:`Update`
      (`SceneComponent.K2_SetRelativeRotation` (`self.leverHandle`) (`KismetMathLibrary.MakeRotator` 0.0 _rotationtimer) false false)
      (`/Engine/EditorBlueprintResources/StandardMacros.CompareFloat` _rotationtimer -90.0
        (:`==`
          (set `self.Click` true))
        (:`<`
          _))
      (`self.Action`))))

(event `self.LeaveClick`
  ;[1 1 1] クリックするとレバーが動くよ！
  (if (`self.Click`)
    (set `self.Clicked` true)
    (goto _label :!via `Reverse`)
    (else
      (goto _label :!via `Reverse`))))

(event `ActorDestroy`
  ;[1 1 1] アクターの削除
  (`self.K2_DestroyActor`))

(fn `UserConstructionScript`)