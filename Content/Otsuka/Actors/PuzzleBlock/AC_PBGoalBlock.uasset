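; Goal puzzle block that acts as a beam receiver, starting an elevator floor when a beam hits it.
; Its construction script caches every BP_ElevatorFloor in the level.
; A beam hit records the caller, sets the beam flag and triggers movement on only the first cached floor.
; Beam deactivation runs the parent logic and sets the cube mesh to FirstBlock, without signalling the elevator.
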(event `self.HitBeam`
  (params (callBy :type "/Game/Otsuka/Actors/PuzzleBlock/AC_PuzzleBlock Object Reference"))
  (bind _elevetorflooraddresses (`self.ElevetorFloorAddresses`))
  ;[1 1 1] ビームを受光口に受けたときに呼び出すイベント
  (set `self.callBy` callBy)
  (set `self.beamFlg` true)
  (`/Game/Otsuka/BluePrints/BML_ArrayMacroLibrary.IsValid` _elevetorflooraddresses
    (:`IsValid`
      (`/Game/hasegawa/Blueprints/BP_ElevatorFloor.MoveStart_Event` (`KismetArrayLibrary.Array_Get` _elevetorflooraddresses)))))

(event `self.DeactiveBeam`
  (`parent.DeactiveBeam`)
  (`/Game/Otsuka/Actors/PuzzleBlock/BML_PuzzleBlockMacros.ChangePBStaticMesh` (`self.Qube`) (`self.firstBlock`)))

(fn `UserConstructionScript`
  (`parent.UserConstructionScript`)
  (bind _outactors (`GameplayStatics.GetAllActorsOfClass` "/Game/hasegawa/Blueprints/BP_ElevatorFloor.BP_ElevatorFloor_C"))
  (set `self.ElevetorFloorAddresses` _outactors))