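; L-shaped (corner) puzzle block, a child of a puzzle block base, that orients its turn pattern from sender and receiver directions.
; On init it picks a left-to-down or right-to-down mesh and sets pitch in quarter turns from the sender's enum value.
; The two enum wrap-around cases are handled explicitly; invalid pairs become a plain cube.
; The construction script caches the original mesh and shows the vanish mesh; init re-caches valid corner meshes.
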(event `self.EV_PuzzleBlockInit`
  (params (SenderDirection :type "/Game/Otsuka/BluePrints/ENU_LightCoord Enum" :default "NewEnumerator0") (ReciverDirection :type "/Game/Otsuka/BluePrints/ENU_LightCoord Enum" :default "NewEnumerator0") (IsVanished :type Boolean))
  (bind _returnvalue (`self.MakeCubeRotatorByPitch` 180.0))
  (bind _returnvalue_2 (`self.MakeCubeRotatorByPitch` 90.0))
  (bind _qube (`self.Qube`))
  (bind _qube_2 (`self.Qube`))
  (bind _returnvalue_3 (`self.MakeCubeRotatorByPitch` (* (`KismetMathLibrary.Conv_ByteToInt` (- (`self.sendCoord`) (enumliteral `/Game/Otsuka/BluePrints/ENU_LightCoord` "NewEnumerator3"))) 90.0)))
  (bind _returnvalue_4 (`self.MakeCubeRotatorByPitch` (* (`KismetMathLibrary.Conv_ByteToInt` (- (`self.sendCoord`) (enumliteral `/Game/Otsuka/BluePrints/ENU_LightCoord` "NewEnumerator3"))) 90.0)))
  (`parent.EV_PuzzleBlockInit` SenderDirection ReciverDirection false)
  ;[1 1 1] ブロックの絵柄の回転を行う
  ;;[1 1 1] 上から右方向の場合（定数値の問題で例外的に処理）
  (if (`self.IsDirecExceptionCase` "NewEnumerator2" "NewEnumerator0")
    (`StaticMeshComponent.SetStaticMesh` _qube "/Game/Kuno/mesh/block_RtoD.block_RtoD")
    (set `self.rot_pitch` _returnvalue_2)
    (`SceneComponent.K2_SetRelativeRotation` _qube _returnvalue_2 false false)
    (set `self.firstBlock` (`StaticMeshComponent.StaticMesh` (`self.Qube`)) :!label _label)
    (else
      ;;[1 1 1] 右から上方向の場合（例外的処理）
      (if (`self.IsDirecExceptionCase` "NewEnumerator0" "NewEnumerator2")
        (`StaticMeshComponent.SetStaticMesh` _qube_2 "/Game/Kuno/mesh/block_LtoD.block_LtoD")
        (set `self.rot_pitch` _returnvalue)
        (`SceneComponent.K2_SetRelativeRotation` _qube_2 _returnvalue false false)
        (goto _label)
        (else
          ;;[1 1 1] 左から下方向のブロックの場合
          (if (== (`self.sendCoord`) (+ (`self.reciveCoord`) 1))
            (`StaticMeshComponent.SetStaticMesh` (`self.Qube`) "/Game/Kuno/mesh/block_LtoD.block_LtoD")
            (set `self.rot_pitch` _returnvalue_3)
            (`SceneComponent.K2_SetRelativeRotation` (`self.Qube`) _returnvalue_3 false false)
            (goto _label)
            (else
              ;;[1 1 1] 右から下方向のブロックの場合
              (if (== (`self.sendCoord`) (- (`self.reciveCoord`) 1))
                (`StaticMeshComponent.SetStaticMesh` (`self.Qube`) "/Game/Kuno/mesh/block_RtoD.block_RtoD")
                (set `self.rot_pitch` _returnvalue_4)
                (`SceneComponent.K2_SetRelativeRotation` (`self.Qube`) _returnvalue_4 false false)
                (goto _label)
                (else
                  ;;[1 1 1] 本来生成されないはずの方向の場合、
                  ;; ただのキューブにする
                  (`StaticMeshComponent.SetStaticMesh` (`self.Qube`) "/Engine/BasicShapes/Cube.Cube"))))))))))

(fn `UserConstructionScript`
  (`parent.UserConstructionScript`)
  (set `self.firstBlock` (`StaticMeshComponent.StaticMesh` (`self.Qube`)))
  (`/Game/Otsuka/Actors/PuzzleBlock/BML_PuzzleBlockMacros.ChangePBStaticMesh` (`self.Qube`) (`self.vanishBlock`)))