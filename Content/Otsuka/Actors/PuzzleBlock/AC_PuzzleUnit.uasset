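; Puzzle unit actor that pairs a wall and a device as child actors and supports spawning puzzle blocks.
; On BeginPlay it binds the spawn-block event and sets both child actor classes from variables.
; The spawn handler adds a child actor component of the supplied class to PuzzleDeviceActor.
; The assignment of PuzzleDeviceActor from the device's child actor is disconnected, so this graph never sets that reference.
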(event `self.ReceiveBeginPlay`
  (add `self.EV_SpawnPuzzleBlock` (delegate `SpawnPuzzleBlock`))
  (`ChildActorComponent.SetChildActorClass` (`self.PuzzleWall`) (`self.SpawnPuzzleWall`))
  (`ChildActorComponent.SetChildActorClass` (`self.PuzzleDevice`) (`self.SpawnPuzzleDevice`)))

(event `SpawnPuzzleBlock` :!signature `self.EV_SpawnPuzzleBlock`
  (params (NewParam :type "Actor Class Reference"))
  (bind _returnvalue (`AddComponent|NODE_AddChildActorComponent-0` :`self` (`self.PuzzleDeviceActor`)))
  (`ChildActorComponent.SetChildActorClass` _returnvalue NewParam))

(fn `UserConstructionScript`)