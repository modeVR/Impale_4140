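; AC_PuzzleViewer is a work-in-progress actor for displaying puzzle block placement on a grid.
; Initialization builds an X-by-Y grid of AC_VacuumPoint through PuzzleResize.
; Incoming blocks are added or updated in parallel arrays of block addresses and spawn data.
; Display is unfinished: CreateViewerBlock only adds a child actor component, reload is empty, grid-positioning logic is disconnected, and Tick loops without effect.
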(event `self.ReceiveTick`
  (params (DeltaSeconds :type "Float (single-precision)"))
  (for _ (`self.PuzzleBlockArray`)
    _))

(event `EV_PuzzleViewerInitalize`
  (`self.PuzzleResize`))

(event `EV_addPuzzleBlockArray`
  (params (puzzleBlock :type "/Game/Otsuka/BluePrints/STR_PuzzleBlockViewerStruct Structure"))
  (bind _returnvalue (`KismetArrayLibrary.Array_Find` (`self.PuzzleBlockArray`) puzzleBlock_PuzzleBlockAddress_5_FDFA58164FA0AD676106EFB55BEFBB9C))
  (`/Engine/EditorBlueprintResources/StandardMacros.CompareInt` _returnvalue -1 ; パズルブロック配列に追加されているブロックの場合、\nそのブロックを操作する
    (:`>`
      (`KismetArrayLibrary.Array_Set` (`self.PuzzleBlockViewData`) _returnvalue puzzleBlock_SpawnData_2_EE5A292D402A1E6D8D6D6BAF4ACF74B3))
    (:`==`
      ;[1 1 1] パズルブロックの位置データを変更、
      ; パズルブロックのアドレスを格納
      (`KismetArrayLibrary.Array_Add` (`self.PuzzleBlockArray`) puzzleBlock_PuzzleBlockAddress_5_FDFA58164FA0AD676106EFB55BEFBB9C :!label _label)
      (`KismetArrayLibrary.Array_Add` (`self.PuzzleBlockViewData`) puzzleBlock_SpawnData_2_EE5A292D402A1E6D8D6D6BAF4ACF74B3))
    (:`<`
      (goto _label))))

(event `EV_ReloadViewerSingle`
  (params (ArrayIndex :type Integer)))

(event `EV_CreateViewerBlock`
  (`AddComponent|NODE_AddChildActorComponent-0`))

(fn `PuzzleResize`
  (for _index (range (`self.puzBlockYLength`))
    (for _index_2 (range (`self.puzBlockXLength`))
      (`self.CreateBlockVacuumPoint` _index_2 _index "/Game/Otsuka/Actors/VacuumPoint/AC_VacuumPoint.AC_VacuumPoint_C"))))

(fn `UserConstructionScript`)