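; AC_PuzzleUnit is a puzzle assembly actor that pairs a puzzle wall with a puzzle device.
; On authority only, the construction script assigns configurable classes to both child actor components and caches the spawned wall.
; At BeginPlay it binds to the EVSpawnPuzzleBlock dispatcher.
; Each call adds a child actor component on PuzzleDeviceActor using the block class passed by the event.
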(event `self.ReceiveBeginPlay`
  (add `self.EV_SpawnPuzzleBlock` (delegate `SpawnPuzzleBlock`)))

(event `SpawnPuzzleBlock` :!signature `self.EV_SpawnPuzzleBlock`
  (params (NewParam :type "Actor Class Reference"))
  (bind _returnvalue (`AddComponent|NODE_AddChildActorComponent-0` :`self` (`self.PuzzleDeviceActor`)))
  (`ChildActorComponent.SetChildActorClass` _returnvalue NewParam))

(fn `UserConstructionScript`
  (bind _puzzlewall (`self.PuzzleWall`))
  (`/Engine/EditorBlueprintResources/ActorMacros.Switch Has Authority`
    (:`Authority`
      (`ChildActorComponent.SetChildActorClass` _puzzlewall (`self.SpawnPuzzleWall`))
      (set `self.m_PuzzleWall` (cast `/Game/Otsuka/Actors/PuzzleWall/AC_PuzzleWall` (`ChildActorComponent.ChildActor` _puzzlewall) :!pure true))
      (`ChildActorComponent.SetChildActorClass` (`self.PuzzleDevice`) (`self.SpawnPuzzleDevice`)))))