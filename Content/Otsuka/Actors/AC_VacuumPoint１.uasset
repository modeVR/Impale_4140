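; Snap point actor that instantly moves other actors onto its SwapPoint component's world location and orients them, with no sweep.
; VacuumToThis places a target actor there with this actor's own rotation.
; VacuumToThisComponent does the same for the child actor of a passed component, but takes the rotation from this actor's parent component.
; Both events only set the transform; nothing is attached.
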(event `VacuumToThis`
  (params (Target :type "Actor Object Reference"))
  ;[1 1 1] 吸着点への吸着
  (`self.K2_SetActorLocation` Target (`SceneComponent.K2_GetComponentLocation` (`self.SwapPoint`)) false false)
  (`self.K2_SetActorRotation` Target (`self.K2_GetActorRotation` self) false))

(event `VacuumToThisComponent`
  (params (actor :type "ChildActorComponent Object Reference"))
  (bind _childactor (`ChildActorComponent.ChildActor` actor))
  ;[1 1 1] （アクターコンポーネント用）吸着点への吸着
  (`self.K2_SetActorLocation` _childactor (`SceneComponent.K2_GetComponentLocation` (`self.SwapPoint`)) false false)
  (`self.K2_SetActorRotation` _childactor (`SceneComponent.K2_GetComponentRotation` (`self.GetParentComponent` self)) false))

(fn `UserConstructionScript`)