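; AC_VacuumPoint is a snap point on a puzzle wall that holds one draggable puzzle block.
; VacuumToThisComponent moves an incoming block to SwapPoint with the parent component's rotation, recording the block and itself as that block's PreviousVacPoint.
; If another block occupies the point, the newcomer snaps back to its previous point, when valid.
; New placements can optionally report to ParentPuzzleWall, using the Tag as coordinate.
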(event `VacuumToThisComponent`
  (params (actor :type "ChildActorComponent Object Reference") (isAddPuzzleViewer :type Boolean))
  (bind _childactor (`ChildActorComponent.ChildActor` actor))
  (if (== (cast `/Game/Otsuka/BaseBluePrint/BBP_DragAndDropObject` _childactor :!pure true) (`self.AttachedDragObject`))
    (`self.SetRotationAndPositionToThisPoint` _childactor)
    (else
      (bind _attacheddragobject (`self.AttachedDragObject`)
        (:`then`
          (bind _previousvacpoint (`/Game/Otsuka/Actors/PuzzleBlock/AC_IPuzzleBlock.PreviousVacPoint` (cast `/Game/Otsuka/Actors/PuzzleBlock/AC_IPuzzleBlock` (cast `/Game/Otsuka/BaseBluePrint/BBP_DragAndDropObject` _childactor :!pure true) :!pure true))
            (:`then`
              (`self.VacuumToThisComponent` _previousvacpoint actor false))
            (:`else`)))
        (:`else`
          (`self.SetRotationAndPositionToThisPoint` _childactor)
          (bind _asac_ipuzzle_block (cast `/Game/Otsuka/Actors/PuzzleBlock/AC_IPuzzleBlock` (`self.AttachedDragObject`))
            (:`then`
              (bind _previousvacpoint_2 (`/Game/Otsuka/Actors/PuzzleBlock/AC_IPuzzleBlock.PreviousVacPoint` _asac_ipuzzle_block)
                (:`then`
                  (`self.ClearAttachedDragObject` _previousvacpoint_2))
                (:`else`
                  _)))
            (:`CastFailed`
              _))
          (bind _asac_ipuzzle_block_2 (cast `/Game/Otsuka/Actors/PuzzleBlock/AC_IPuzzleBlock` _childactor)
            (:`then`
              (set `/Game/Otsuka/Actors/PuzzleBlock/AC_IPuzzleBlock.PreviousVacPoint` self _asac_ipuzzle_block_2))
            (:`CastFailed`
              _))
          (set `self.AttachedDragObject` (cast `/Game/Otsuka/BaseBluePrint/BBP_DragAndDropObject` _childactor :!pure true))
          (if isAddPuzzleViewer
            (`self.ReloadPuzzleViewer_1_Event` null)))))))

(event `ClearAttachedDragObject`
  (set `self.AttachedDragObject` null))

(event `CustomEvent_0`)

(event `ReloadPuzzleViewer_1_Event`
  (params (InputPin :type "Actor Object Reference"))
  (bind _parentpuzzlewall (`self.ParentPuzzleWall`)
    (:`then`
      (`/Game/Otsuka/Actors/PuzzleWall/AC_PuzzleWall.EV_SetPuzzleBlock` _parentpuzzlewall InputPin (`self.Tag`)))
    (:`else`)))

(fn `ReloadPuzzleViewer`
  (params (InputPin :type "Actor Object Reference")))

(fn `SetRotationAndPositionToThisPoint`
  (params (self2 :type "Actor Object Reference"))
  (`self.K2_SetActorLocation` self2 (`SceneComponent.K2_GetComponentLocation` (`self.SwapPoint`)) false false)
  (`self.K2_SetActorRotation` self2 (`SceneComponent.K2_GetComponentRotation` (`self.GetParentComponent` self)) false))

(fn `UserConstructionScript`)