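; AC_DustPoint is an actor with a vacuum event that repositions puzzle blocks.
; VacuumtoThisComponent casts the passed-in object's child actor to AC_PuzzleBlock, then sets that block's root to the world location of its SpawnVacPoint's SwapPoint.
; The destination comes from the block's own reference, and the move is instant, with no sweep.
; BeginPlay and the construction script only call their parents.
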(event `self.ReceiveBeginPlay`
  (`parent.ReceiveBeginPlay`))

(event `self.VacuumToThisComponent`
  (params (actor :type "ChildActorComponent Object Reference"))
  (bind _asac_puzzle_block (cast `/Game/Otsuka/Actors/PuzzleBlock/AC_PuzzleBlock` (`ChildActorComponent.ChildActor` actor)))
  (`SceneComponent.K2_SetWorldLocation` (`/Game/Otsuka/BaseBluePrint/BBP_ClickableObject.Root` _asac_puzzle_block) (`SceneComponent.K2_GetComponentLocation` (`/Game/Otsuka/Actors/VacuumPoint/AC_VacuumPoint.SwapPoint` (`/Game/Otsuka/Actors/PuzzleBlock/AC_PuzzleBlock.SpawnVacPoint` _asac_puzzle_block))) false false))

(fn `UserConstructionScript`
  (`parent.UserConstructionScript`))