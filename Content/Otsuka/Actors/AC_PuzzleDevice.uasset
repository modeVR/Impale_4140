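; AC_PuzzleDevice is a puzzle device actor that builds a vertical stack of puzzle blocks from SpawnBlockList.
; Its construction script adds a child actor per block ID, spaced along Z by block size and spawn step.
; Each block gets a co-located AC_VacuumPoint child, rotated 180 degrees and stored as that block's SpawnVacPoint.
; The event graph is empty, so all logic runs at construction.
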(fn `UserConstructionScript`
  (locals (CounterI :type Integer))
  (for _index (range (`KismetArrayLibrary.Array_Length` (`self.SpawnBlockList`)))
    (bind _output_get (set `local.CounterI` _index))
    (bind _returnvalue (`AddComponent|NODE_AddChildActorComponent-0`))
    (`ChildActorComponent.SetChildActorClass` _returnvalue (`/Game/Otsuka/Actors/GetActorClassFromBlockID.GetActorClassFromBlockID` (`KismetArrayLibrary.Array_Get` (`self.SpawnBlockList`) (`local.CounterI`))))
    (bind _returnvalue_2 (`KismetMathLibrary.MakeVector` 0.0 0.0 (* _output_get (- (+ (`self.BlockSize`) (`self.BlockSpawnYStep`)) -1.0))))
    (`SceneComponent.K2_SetRelativeLocation` _returnvalue _returnvalue_2 false false)
    (bind _returnvalue_3 (`AddComponent|NODE_AddChildActorComponent-1`))
    (`ChildActorComponent.SetChildActorClass` _returnvalue_3 "/Game/Otsuka/Actors/VacuumPoint/AC_VacuumPoint.AC_VacuumPoint_C")
    (`SceneComponent.K2_SetRelativeLocation` _returnvalue_3 _returnvalue_2 false false)
    (`SceneComponent.K2_SetRelativeRotation` _returnvalue_3 (struct :`Yaw` 180.0) false false)
    (set `/Game/Otsuka/Actors/PuzzleBlock/AC_PuzzleBlock.SpawnVacPoint` (cast `/Game/Otsuka/Actors/VacuumPoint/AC_VacuumPoint` (`ChildActorComponent.ChildActor` _returnvalue_3) :!pure true) (cast `/Game/Otsuka/Actors/PuzzleBlock/AC_PuzzleBlock` (`ChildActorComponent.ChildActor` _returnvalue) :!pure true))))