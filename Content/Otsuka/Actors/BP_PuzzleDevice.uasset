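; BP_PuzzleDevice is a puzzle board actor that lays out a vertical grid of child actors, cast to AC_SwapPoint.
; The construction script loops over the configurable block X and Y lengths, adding each child from the VacuumPointLeftTop transform.
; It then positions each in the XZ plane using the SwapRange box extent plus step spacing, with Y offset by that extent.
; The event graph holds no active logic.
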(fn `UserConstructionScript`
  (locals (counterI :type Integer) (counterJ :type Integer))
  (for _index (range (`self.puzBlockXLength`))
    (set `local.counterJ` _index)
    (for _index_2 (range (`self.puzBlockYLength`))
      (set `local.counterI` _index_2)
      (bind _returnvalue (`AddComponent|NODE_AddChildActorComponent-0` :`RelativeTransform` (`SceneComponent.GetRelativeTransform` (`self.VacuumPointLeftTop`))))
      (bind (_returnvalue_x _returnvalue_y _returnvalue_z) (`KismetMathLibrary.BreakVector` (`BoxComponent.GetScaledBoxExtent` (`/Game/Otsuka/BluePrints/AC_SwapPoint.SwapRange` (cast `/Game/Otsuka/BluePrints/AC_SwapPoint` (`ChildActorComponent.ChildActor` _returnvalue) :!pure true)))))
      (`SceneComponent.K2_SetRelativeLocation` _returnvalue (`KismetMathLibrary.MakeVector` (* (`local.counterI`) (+ (`self.puzVacuumXStep`) _returnvalue_x)) _returnvalue_y (* (`local.counterJ`) (+ _returnvalue_z (`self.puzVacuumYStep`)))) false false))))