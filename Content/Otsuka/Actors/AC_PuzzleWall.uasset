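; AC_PuzzleWall is a puzzle board actor that lays out a grid of vacuum points and places the initial puzzle blocks on them.
; The construction script creates the points as child actors spaced by their swap-range extents, plus a dust point left of the grid.
; It spawns listed blocks at their tagged points, records each one's spawn point and caches the start block.
; A raycast-from-start event makes that start block change its particle target.
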(event `self.ReceiveBeginPlay`
  (add `self.EV_LaycastFromStart` (delegate `Laycast FromStart`)))

(event `Laycast FromStart`
  (`/Game/Otsuka/Actors/PuzzleBlock/AC_PuzzleBlock.ChangeParticleTarget` (`self.StartBlock`)))

(fn `CreateBlockVacuumPoint`
  (params (x :type Integer) (y :type Integer) (CreateActor :type "Actor Class Reference") (isAddArray :type Boolean))
  (locals (counterJ :type Integer) (counterI :type Integer) (t_isAddArray :type Boolean))
  (set `local.counterI` x)
  (set `local.counterJ` y)
  (set `self.NewVar_0` CreateActor)
  (set `local.t_isAddArray` isAddArray)
  (bind _returnvalue (`AddComponent|NODE_AddChildActorComponent-0` :`RelativeTransform` (`SceneComponent.GetRelativeTransform` (`self.VacuumPointLeftTop`))))
  (`ChildActorComponent.SetChildActorClass` _returnvalue (`self.NewVar_0`))
  (if (`local.t_isAddArray`)
    (bind _asac_vacuum_point (cast `/Game/Otsuka/Actors/VacuumPoint/AC_VacuumPoint` (`ChildActorComponent.ChildActor` _returnvalue) :!pure true))
    (`KismetArrayLibrary.Array_Add` (`self.VacuumPointArray`) _asac_vacuum_point))
  (bind (_returnvalue_x _returnvalue_y _returnvalue_z) (`KismetMathLibrary.BreakVector` (`BoxComponent.GetScaledBoxExtent` (`/Game/Otsuka/Actors/VacuumPoint/AC_VacuumPoint.SwapRange` _asac_vacuum_point))))
  (`SceneComponent.K2_SetRelativeLocation` _returnvalue (`KismetMathLibrary.MakeVector` (* (`local.counterI`) (+ (`self.puzVacuumXStep`) _returnvalue_x)) _returnvalue_y (* (`local.counterJ`) (+ _returnvalue_z (`self.puzVacuumYStep`)))) false false))

(fn `UserConstructionScript`
  (locals (CounterI :type Integer) (CounterJ :type Integer))
  (bind _item (`KismetArrayLibrary.Array_Get` (`self.SpawnBlockList`) (`local.CounterI`)))
  (bind _item_2 (`KismetArrayLibrary.Array_Get` (`self.VacuumPointArray`) (+ (- (break `/Game/Otsuka/BluePrints/STR_VacuumPointTag` (break `/Game/Otsuka/Actors/STR_PBSpawnData` _item)) 1) (* (- (`.TagY_4_9AB4ECBF49B4FA7F72CC04A2CA904E19` (break `/Game/Otsuka/BluePrints/STR_VacuumPointTag` (break `/Game/Otsuka/Actors/STR_PBSpawnData` _item))) 1) (`self.puzBlockXLength`)))))
  (for _index (range (`self.puzBlockYLength`))
    (set `local.CounterJ` _index)
    (for _index_2 (range (`self.puzBlockXLength`))
      (set `local.CounterI` _index_2)
      (`self.CreateBlockVacuumPoint` (`local.CounterI`) (`local.CounterJ`) "/Game/Otsuka/Actors/VacuumPoint/AC_VacuumPoint.AC_VacuumPoint_C" true))
    ;[1 1 1] 初期配置ブロックの生成
    (for _index_3 (range (`KismetArrayLibrary.Array_Length` (`self.SpawnBlockList`)))
      (set `local.CounterI` _index_3)
      (bind _returnvalue (`AddComponent|NODE_AddChildActorComponent-1`))
      (`ChildActorComponent.SetChildActorClass` _returnvalue (`/Game/Otsuka/Actors/GetActorClassFromBlockID.GetActorClassFromBlockID` (`.SpawnBlockID_6_5AE4D29D4A8A0886F30E0CAE354F833F` (break `/Game/Otsuka/Actors/STR_PBSpawnData` _item))))
      (if (`|EnumEquality` (`.SpawnBlockID_6_5AE4D29D4A8A0886F30E0CAE354F833F` (break `/Game/Otsuka/Actors/STR_PBSpawnData` _item)) "NewEnumerator1")
        (set `self.StartBlock` (cast `/Game/Otsuka/Actors/PuzzleBlock/AC_PuzzleBlock` (`ChildActorComponent.ChildActor` _returnvalue) :!pure true)))
      (`SceneComponent.K2_SetWorldLocation` _returnvalue (`SceneComponent.K2_GetComponentLocation` (`/Game/Otsuka/Actors/VacuumPoint/AC_VacuumPoint.SwapPoint` _item_2)) false false)
      (set `/Game/Otsuka/Actors/PuzzleBlock/AC_PuzzleBlock.SpawnVacPoint` _item_2 (cast `/Game/Otsuka/Actors/PuzzleBlock/AC_PuzzleBlock` (`ChildActorComponent.ChildActor` _returnvalue) :!pure true)))
    (`self.CreateBlockVacuumPoint` -1 0 "/Game/Otsuka/Actors/VacuumPoint/AC_DustPoint.AC_DustPoint_C")))