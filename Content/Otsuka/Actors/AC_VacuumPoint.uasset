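; AC_VacuumPoint is an actor that acts as a snap destination, instantly moving objects passed to it onto its SwapPoint component's world location.
; VacuumToThis places a target actor there and matches it to this actor's rotation.
; VacuumToThisComponent does the same for a child actor component's spawned actor, but takes rotation from this actor's parent component.
; Both moves are unswept, and BeginPlay, overlap and Tick are empty.
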(event `self.ReceiveBeginPlay`)

(event `VacuumToThis`
  (params (Target :type "Actor Object Reference"))
  (`self.K2_SetActorLocation` Target (`SceneComponent.K2_GetComponentLocation` (`self.SwapPoint`)) false false)
  (`self.K2_SetActorRotation` Target (`self.K2_GetActorRotation` self) false))

(event `VacuumToThisComponent`
  (params (actor :type "ChildActorComponent Object Reference"))
  (bind _childactor (`ChildActorComponent.ChildActor` actor))
  (`self.K2_SetActorLocation` _childactor (`SceneComponent.K2_GetComponentLocation` (`self.SwapPoint`)) false false)
  (`self.K2_SetActorRotation` _childactor (`SceneComponent.K2_GetComponentRotation` (`self.GetParentComponent` self)) false))

(fn `UserConstructionScript`)