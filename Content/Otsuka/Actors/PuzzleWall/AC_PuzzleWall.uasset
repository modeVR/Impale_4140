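; Puzzle wall actor for a laser-beam block puzzle, holding a grid of snap points for blocks.
; On authority, the construction script builds the vacuum-point grid as child actors, spawns and snaps preset blocks, registers them with the puzzle viewer and adds a trash point.
; BeginPlay passes a buffered spawn list to the GameInstance.
; Events re-fire beams from start blocks, register placed blocks, and report goal completion to the parent PuzzleUnit through a closing gate.
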(event `self.ReceiveBeginPlay`
  (bind _output_get (set `self.gameInstance` (`/Game/Otsuka/BluePrints/BML_GameInstanceMacro.GetGameInstanceKUNO`)))
  (for _array_element (`self.Buf_SpawNBlockList`)
    (`/Game/Kuno/BluePrint/BP_ImpaleInstanceKUNO.EV_AddSpawnBlockList` _output_get _array_element)))

(event `EV_LaycastFromStartBlock_Event`
  ;[1 1 1] スタート地点からのレーザー射出
  (`KismetSystemLibrary.PrintString` "laycaststart")
  (`/Game/Otsuka/Actors/PuzzleBlock/AC_IPuzzleBlock.DeactiveBeam` (`self.NewVar_1`))
  (for _array_element (`self.StartPuzzleBlock`)
    (`/Game/Otsuka/Actors/PuzzleBlock/AC_IPuzzleBlock.ChangeParticleTarget` _array_element)))

(event `EV_OnGoal`
  ;[1 1 1] ゴール時のイベントをUnitに送信
  (`|ExecutionSequence`
    (:`then_0`
      (`/Engine/EditorBlueprintResources/StandardMacros.Gate` false :!label _label
        (:`Exit`
          (`/Game/Otsuka/Actors/PuzzleUnit/AC_PuzzleUnitWithViewer.EV_OnGoal` (`self.ParentUnit`)))))
    (:`then_1`
      (goto _label :!via `Close`))))

(event `EV_SetPuzzleBlock`
  (params (SetActor :type "Actor Object Reference") (VacCoord :type "/Game/Otsuka/BluePrints/STR_VacuumPointTag Structure"))
  (bind _asac_ipuzzle_block (cast `/Game/Otsuka/Actors/PuzzleBlock/AC_IPuzzleBlock` SetActor))
  (bind _puzzleviewer (`self.PuzzleViewer`)
    (:`then`
      (`/Game/Otsuka/Actors/AC_PuzzleViewer.AddPuzzleBlockArray` _puzzleviewer (make `/Game/Otsuka/BluePrints/STR_PuzzleBlockViewerStruct` _asac_ipuzzle_block (make `/Game/Otsuka/Actors/STR_PBSpawnData` VacCoord)) false))
    (:`else`)))

(fn `CreateBlockVacuumPoint`
  (params (x :type Integer) (y :type Integer) (CreateActor :type "Actor Class Reference") (isAddArray :type Boolean))
  (locals (counterJ :type Integer) (counterI :type Integer) (t_isAddArray :type Boolean))
  (set `local.counterI` x)
  (set `local.counterJ` y)
  (set `self.NewVar_0` CreateActor)
  (set `local.t_isAddArray` isAddArray)
  (bind _returnvalue (`AddComponent|NODE_AddChildActorComponent-0` :`RelativeTransform` (`SceneComponent.GetRelativeTransform` (`self.VacuumPointLeftTop`))))
  (`ChildActorComponent.SetChildActorClass` _returnvalue (`self.NewVar_0`))
  (if (`local.t_isAddArray`)
    (bind _asac_vacuum_point (cast `/Game/Otsuka/Actors/VacuumPoint/AC_VacuumPoint` (`ChildActorComponent.ChildActor` _returnvalue) :!pure true))
    (`KismetArrayLibrary.Array_Add` (`self.VacuumPointArray`) _asac_vacuum_point))
  (set `/Game/Otsuka/Actors/VacuumPoint/AC_VacuumPoint.ParentPuzzleWall` self _asac_vacuum_point)
  (set `/Game/Otsuka/Actors/VacuumPoint/AC_VacuumPoint.Tag` (make `/Game/Otsuka/BluePrints/STR_VacuumPointTag` (+ (`local.counterI`) 1) (+ 1 (`local.counterJ`))) _asac_vacuum_point)
  (bind (_returnvalue_x _returnvalue_y _returnvalue_z) (`KismetMathLibrary.BreakVector` (`BoxComponent.GetScaledBoxExtent` (`/Game/Otsuka/Actors/VacuumPoint/AC_VacuumPoint.SwapRange` _asac_vacuum_point))))
  (`SceneComponent.K2_SetRelativeLocation` _returnvalue (`KismetMathLibrary.MakeVector` (* (`local.counterI`) (+ (`self.puzVacuumXStep`) _returnvalue_x)) _returnvalue_y (* (`local.counterJ`) (+ _returnvalue_z (`self.puzVacuumYStep`)))) false false))

(fn `GetVacPointByPuzzleCoord`
  (params (x :type Integer) (y :type Integer))
  (returns (Item :type "/Game/Otsuka/Actors/VacuumPoint/AC_VacuumPoint Object Reference") (isValid :type Boolean))
  (locals (NewLocalVar_0 :type "/Game/Otsuka/Actors/VacuumPoint/AC_VacuumPoint Object Reference"))
  (bind _returnvalue (and (>= x 1) (>= y 1)))
  (if _returnvalue
    (bind _output_get (set `local.NewLocalVar_0` (`KismetArrayLibrary.Array_Get` (`self.VacuumPointArray`) (+ (- x 1) (* (- y 1) (`self.puzBlockXLength`)))))))
  (return _output_get _returnvalue))

(fn `UserConstructionScript`
  (locals (CounterI :type Integer) (CounterJ :type Integer))
  (bind (_item_spawnpoint _item_spawnblockid _item_senderdirection _item_reciverdirection _item_puzzleblockref _item_correctbeamcolor _item_outputcolor _item_avaliableanycolor) (break `/Game/Otsuka/Actors/STR_PBSpawnData` (`KismetArrayLibrary.Array_Get` (`self.SpawnBlockList`) (`local.CounterI`))))
  (bind _item (`KismetArrayLibrary.Array_Get` (`self.SpawnBlockList`) (`local.CounterI`)))
  (bind _puzzleblockclass (`/Game/Otsuka/Actors/GetActorClassFromBlockID.GetActorClassFromBlockID` (`.SpawnBlockID_6_5AE4D29D4A8A0886F30E0CAE354F833F` (break `/Game/Otsuka/Actors/STR_PBSpawnData` _item))))
  (bind _item_2 (`self.GetVacPointByPuzzleCoord` (break `/Game/Otsuka/BluePrints/STR_VacuumPointTag` (break `/Game/Otsuka/Actors/STR_PBSpawnData` _item)) (`.TagY_4_9AB4ECBF49B4FA7F72CC04A2CA904E19` (break `/Game/Otsuka/BluePrints/STR_VacuumPointTag` (break `/Game/Otsuka/Actors/STR_PBSpawnData` _item)))))
  (`/Engine/EditorBlueprintResources/ActorMacros.Switch Has Authority`
    (:`Authority`
      (`|ExecutionSequence`
        (:`then_0`
          ;[1 1 1] パズルビューワーの取得
          (bind _asac_puzzle_unit_with_viewer (cast `/Game/Otsuka/Actors/PuzzleUnit/AC_PuzzleUnitWithViewer` (`self.GetParentActor`)))
          (bind _asac_puzzle_viewer (cast `/Game/Otsuka/Actors/AC_PuzzleViewer` (`ChildActorComponent.ChildActor` (`/Game/Otsuka/Actors/PuzzleUnit/AC_PuzzleUnitWithViewer.PuzzleViewer` _asac_puzzle_unit_with_viewer))))
          (set `self.PuzzleViewer` _asac_puzzle_viewer))
        (:`then_1`
          ;[1 1 1] ゲームインスタンスの取得
          (set `self.gameInstance` (`/Game/Otsuka/BluePrints/BML_GameInstanceMacro.GetGameInstanceKUNO`))
          ;[1 1 1] 親Unitの取得
          (bind _asac_puzzle_unit (cast `/Game/Otsuka/Actors/PuzzleUnit/AC_PuzzleUnit` (`self.GetParentActor`)))
          (set `self.ParentUnit` _asac_puzzle_unit))
        (:`then_2`
          (`|ExecutionSequence`
            (:`then_0`
              ;[1 1 1] 吸着点の作成
              (for _index (range (`self.puzBlockYLength`))
                (set `local.CounterJ` _index)
                (for _index_2 (range (`self.puzBlockXLength`))
                  (set `local.CounterI` _index_2)
                  (`self.CreateBlockVacuumPoint` (`local.CounterI`) (`local.CounterJ`) "/Game/Otsuka/Actors/VacuumPoint/AC_VacuumPoint.AC_VacuumPoint_C" true))))
            (:`then_1`
              ;[1 1 1] 初期配置ブロックの生成
              (for (_ _array_index) (`self.SpawnBlockList`)
                (set `local.CounterI` _array_index)
                (`|ExecutionSequence`
                  (:`then_0`
                    (bind _returnvalue (`AddComponent|NODE_AddChildActorComponent-1`))
                    (`ChildActorComponent.SetChildActorClass` _returnvalue _puzzleblockclass)
                    (if (== _puzzleblockclass "/Game/Otsuka/Actors/PuzzleBlock/AC_PBStartBlock.AC_PBStartBlock_C")
                      (bind _childactor (`ChildActorComponent.ChildActor` _returnvalue))
                      (`/Game/Otsuka/Actors/PuzzleBlock/AC_IPuzzleBlock.ChangeBeamColor` (cast `/Game/Otsuka/Actors/PuzzleBlock/AC_IPuzzleBlock` _childactor :!pure true) (`.OutputColor_24_97FFE6344AE582212A5A7BA18ACA19A7` (break `/Game/Otsuka/Actors/STR_PBSpawnData` _item))))
                    (`/Game/Otsuka/Actors/VacuumPoint/AC_VacuumPoint.VacuumToThisComponent` _item_2 _returnvalue false)
                    (bind _asac_ipuzzle_block (cast `/Game/Otsuka/Actors/PuzzleBlock/AC_IPuzzleBlock` _childactor :!pure true))
                    (set `/Game/Otsuka/Actors/PuzzleBlock/AC_IPuzzleBlock.SpawnVacPoint` _item_2 _asac_ipuzzle_block)
                    (if (`|EnumEquality` (`.SpawnBlockID_6_5AE4D29D4A8A0886F30E0CAE354F833F` (break `/Game/Otsuka/Actors/STR_PBSpawnData` _item)) "NewEnumerator1")
                      (`KismetArrayLibrary.Array_Add` (`self.StartPuzzleBlock`) _asac_ipuzzle_block)))
                  (:`then_1`
                    ;;[1 1 1] パズルブロックの初期化処理＆壁のブロックリストに登録
                    (`/Game/Otsuka/Actors/PuzzleBlock/AC_IPuzzleBlock.EV_PuzzleBlockInit` _asac_ipuzzle_block (`.SenderDirection_11_4B5ECC314010BE07A88BD5A95DC771EC` (break `/Game/Otsuka/Actors/STR_PBSpawnData` _item)) (`.ReciverDirection_12_FEF3A18648801EEA4AF6A1901E58683E` (break `/Game/Otsuka/Actors/STR_PBSpawnData` _item)) true (`.AvaliableAnyColor_21_7AF6BBBD408EE8970122B596A1457918` (break `/Game/Otsuka/Actors/STR_PBSpawnData` _item)) (`.correctBeamColor_19_6031F2DA4E65E4AD47152997FF9126E3` (break `/Game/Otsuka/Actors/STR_PBSpawnData` _item)) (`.OutputColor_24_97FFE6344AE582212A5A7BA18ACA19A7` (break `/Game/Otsuka/Actors/STR_PBSpawnData` _item)))
                    (set `/Game/Otsuka/BaseBluePrint/BBP_ClickableObject.IsAcsessable` false _asac_ipuzzle_block)
                    (`KismetArrayLibrary.Array_Add` (`self.NewVar_1`) _asac_ipuzzle_block)
                    ;;[1 1 1] ブロックビューワーのブロックリストに
                    ;; パズルブロックを登録
                    (bind _puzzleviewer (`self.PuzzleViewer`)
                      (:`then`
                        (`/Game/Otsuka/Actors/AC_PuzzleViewer.AddPuzzleBlockArray` _puzzleviewer (make `/Game/Otsuka/BluePrints/STR_PuzzleBlockViewerStruct` _asac_ipuzzle_block (make `/Game/Otsuka/Actors/STR_PBSpawnData` _item_spawnpoint _item_spawnblockid _item_senderdirection _item_reciverdirection null _item_correctbeamcolor _item_outputcolor _item_avaliableanycolor)) true))
                      (:`else`))))))
            (:`then_2`
              (`self.CreateBlockVacuumPoint` -1 0 "/Game/Otsuka/Actors/VacuumPoint/AC_DustPoint.AC_DustPoint_C") ; ゴミ箱の作成
              ;[1 1 1] L字形ブロックのビームを無力化
              (for _array_element (`self.NewVar_1`)
                (bind _asac_pb_lblock (cast `/Game/Otsuka/Actors/PuzzleBlock/AC_PB_LBlock` _array_element))
                (`/Game/Otsuka/Actors/PuzzleBlock/AC_IPuzzleBlock.DeactiveBeam` _asac_pb_lblock)))))))))